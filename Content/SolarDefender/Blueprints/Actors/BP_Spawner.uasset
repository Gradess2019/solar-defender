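; BP_Spawner is an actor that repeatedly spawns BP_AIPawn enemies within its Box component, starting at BeginPlay.
; An endless Delay loop waits the inverse of SpawnRate times a random factor before each spawn.
; Location is the box center offset by its extent times a single random scalar, so points fall along one diagonal.
; Spawns are skipped when colliding, and new pawns take the spawner's rotation.
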(event Custom|SpawnEnemy
  (bind _box (Variables|Default|GetBox))
  (bind (_origin _boxextent) (Collision|GetComponentBounds _box))
  (bind _returnvalue (Game|SpawnActorfromClass "/Game/SolarDefender/Blueprints/Pawns/BP_AIPawn.BP_AIPawn_C" (Math|Transform|MakeTransform (+ _origin (* _boxextent (Math|Random|RandomFloatinRange -1.0 1.0))) "0, 0, 0" "1,1,1") "DontSpawnIfColliding" 0 0))
  (Transformation|SetActorRotation _returnvalue (Transformation|GetActorRotation)))

(event EventBeginPlay
  (Utilities|FlowControl|Delay (* (/ 1.0 (Variables|Default|GetSpawnRate)) (Math|Random|RandomFloatinRange 0.25 3.0)) :!label _label)
  (CallFunction|SpawnEnemy)
  (goto _label))

(fn ConstructionScript)