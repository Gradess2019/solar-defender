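; Endless world generator that strings BP_Tile actors along X as attached children, following the scene root reported by BP_SceneRootFinder.
; BeginPlay spawns an initial batch and starts a looping timer for periodic checks.
; Each tile is a seeded random TilesData pick, async-loaded and offset by actor bounds.
; The location check destroys the last attached tile when distant and spawns another as the root nears the +X edge.
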(event OnSceneRootFound(BP_SceneRootFinder)
  (params (SceneRoot :type BP%20Scene%20Root%20Object%20Reference))
  (Variables|Default|SetScene%20Root SceneRoot))

(event Custom|DirectSpawnTile
  (if (Utilities|Array|IsNotEmpty (Variables|Generation|Spawn|GetTilesData))
    (Utilities|SpawnTile)))

(event Custom|DirectSpawnTiles
  (params (Num :type Integer))
  (if (Utilities|Array|IsNotEmpty (Variables|Generation|Spawn|GetTilesData))
    (Utilities|SpawnTiles Num)))

(event Custom|CheckSceneRootLocation
  (bind _outactors (Actor|GetAttachedActors false))
  (bind _returnvalue (Utilities|Array|LastIndex _outactors))
  (bind _output (Utilities|Array|Get(acopy) _outactors _returnvalue))
  (Utilities|IsValid (Variables|Default|GetScene%20Root)
    (:Is%20Valid
      (bind (_center _boxextent) (Collision|GetActorArrayBounds (Actor|GetAttachedActors false)))
      (Utilities|FlowControl|Sequence
        (:then_0
          (if (> (Class|Actor|GetSquaredHorizontalDistanceto (Variables|Default|GetScene%20Root) _output) 1e+06)
            (Actor|DestroyActor _output)))
        (:then_1
          (if (< (Class|KismetMathLibrary|VectorDistanceSquared (Math|Vector|MakeVector (+ (.X (Math|Vector|BreakVector _center)) (.x _boxextent)) (.Y (Math|Vector|BreakVector _center)) (.Z (Math|Vector|BreakVector _center))) (Transformation|GetActorLocation (Variables|Default|GetScene%20Root))) (Variables|Generation|Spawn|GetSquaredMinDistance))
            (Utilities|SpawnTile)))))))

(event EventBeginPlay
  (Utilities|Time|SetTimerbyEvent (EventDispatchers|CreateEvent :!event Custom|CheckSceneRootLocation) 0.1 true)
  (CallFunction|DirectSpawnTiles (Variables|Generation|Spawn|GetNum)))

(fn ConstructionScript)