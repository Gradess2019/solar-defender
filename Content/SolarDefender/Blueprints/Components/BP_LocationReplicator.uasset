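; BP_LocationReplicator is a component that shares its owning actor's location through a replicated variable.
; Once Start is called, a looping timer sends the owner's location to ServerUpdateLocation at a configurable interval, which stores it in ReplicatedLocation.
; The RepNotify then fires the LocationReplicated dispatcher with the new position.
; A squared-distance threshold check exists but is unconnected, so updates are sent regardless of movement.
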(event Custom|ServerUpdateLocation
  (params (ActorLocation :type Vector))
  (Variables|Replication|SetReplicatedLocation ActorLocation))

(event Custom|UpdateLocation
  (CallFunction|ServerUpdateLocation (Transformation|GetActorLocation (Components|GetOwner))))

(event Custom|Start
  (Utilities|Time|SetTimerbyEvent (delegate Custom|UpdateLocation) (Variables|Replication|GetLocationUpdateFrequency) true))

(fn OnRepReplicatedLocation
  (Default|CallOnLocationReplicated (Variables|Replication|GetReplicatedLocation)))