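; BP_AIPawn is an AI pawn in SolarDefender that constantly moves along its own forward direction.
; Each tick it feeds GetInput, the actor's forward vector scaled by Speed, into a FloatingPawnMovement component as movement input.
; Tick also accumulates a scaled Time value, which none of the shown graphs use.
; It contains no steering or target logic, and its construction script is empty.
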(event EventTick
  (params (DeltaSeconds :type Float%20%28single-precision%29))
  (Variables|AI|SetTime (+ (* DeltaSeconds 3e+02) (Variables|AI|GetTime)))
  (Class|PawnMovementComponent|AddInputVector (Variables|Default|GetFloatingPawnMovement) (AI|Movement|GetInput) false))

(fn ConstructionScript)

(fn GetInput
  (return (* (Transformation|GetActorForwardVector) (LocalVariables|GetSpeed))))