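; BP_Projectile is a projectile actor for Solar Defender that flies straight along its forward vector.
; On begin play it waits briefly, applies the mesh from its Data variable, then starts an UpdateLocation timeline that offsets it by Data's speed on each update, without sweep.
; A custom event can reapply the mesh.
; An off-screen destroy check exists but is unconnected.
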(event Custom|CustomEvent_0
  (Components|StaticMesh|SetStaticMesh (Variables|Default|GetMesh) (Variables|/Game/SolarDefender/Blueprints/Core/DataAssets/BP_ProjectileDataAsset.BP_ProjectileDataAsset_C|GetMesh (Variables|Default|GetData))))

(event EventBeginPlay
  (Utilities|FlowControl|Delay 0.02)
  (Components|StaticMesh|SetStaticMesh (Variables|Default|GetMesh) (Variables|/Game/SolarDefender/Blueprints/Core/DataAssets/BP_ProjectileDataAsset.BP_ProjectileDataAsset_C|GetMesh (Variables|Default|GetData)))
  (Timeline|UpdateLocation PlayFromStart
    (:Update
      (Transformation|AddActorWorldOffset (* (Transformation|GetActorForwardVector) (Variables|/Game/SolarDefender/Blueprints/Core/DataAssets/BP_ProjectileDataAsset.BP_ProjectileDataAsset_C|GetSpeed (Variables|Default|GetData)))))))

(fn ConstructionScript)