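; Scene root actor for SolarDefender that carries the main camera and is built to scroll through the level.
; On BeginPlay it spawns a CameraActor, snaps it to its SpringArm, registers itself with the GameState and starts the UpdateLocation timeline.
; The timeline's update is meant to offset the actor by SceneSpeed per tick, without sweep or frame-time scaling.
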(event EventBeginPlay
  (SceneRoot|Initialization|InitCamera)
  (Class|BPIGameState|RegisterSceneRoot(Message) (Game|GetGameState) self)
  (Components|Timeline|PlayfromStart (Variables|Default|GetUpdateLocation)))

(fn ConstructionScript)

(fn InitCamera
  (bind _returnvalue (Game|SpawnActorfromClass "/Script/Engine.CameraActor" (Math|Transform|MakeTransform "0, 0, 0" "0, 0, 0" "1,1,1") "AlwaysSpawn" 0 0))
  (Variables|Default|SetMainCamera _returnvalue)
  (Transformation|AttachComponentToComponent (Variables|Default|GetMainCamera) (Variables|Default|GetSpringArm) "None" "SnapToTarget" "SnapToTarget" "KeepWorld" true))