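; Player pawn for SolarDefender with axis-driven floating movement and custom location replication through a location replicator component.
; The locally controlled client starts the replicator, and its replicated location events update a stored target.
; For client-owned pawns, the server hides the cube, removes movement and drives a spawned proxy, while other clients move the pawn itself.
; Timelines act as ticks, lerping toward the target until within a distance threshold.
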(event EventBeginPlay
  ;[1 1 1] Initialization
  (if (Networking|IsServer)
    (if (not (== (Pawn|GetController) (Game|GetPlayerController 0)))
      (Variables|Replication|SetbClient true)
      (CallFunction|ListenLocationReplication))
    (else
      (CallFunction|InitializeClientReplication))))

(event Input|AxisEvents|InputAxisMoveRight
  (params (AxisValue :type Float%20%28single-precision%29))
  (Pawn|Input|AddMovementInput (Transformation|GetActorRightVector) AxisValue false))

(event Input|AxisEvents|InputAxisMoveForward
  (params (AxisValue :type Float%20%28single-precision%29))
  (Pawn|Input|AddMovementInput (Transformation|GetActorForwardVector) AxisValue false))

(event OnLocationReplicated(BP_LocationReplicator)
  (params (NewLocation :type Vector :default "0, 0, 0"))
  (Variables|Replication|SetReplicatedLocation NewLocation))

(event Custom|InitializeClientReplication
  (if (Pawn|IsLocallyControlled)
    (Default|Start (Variables|Default|GetBP_LocationReplicator))
    (elif (Variables|Replication|GetbClient)
      (CallFunction|ListenLocationReplication))))

(event Custom|ListenLocationReplication
  (if (Networking|IsServer)
    (Replication|SpawnProxy)
    (Timeline|Timeline_1 PlayFromStart
      (:Update
        (Replication|UpdateLocation (Variables|Replication|GetProxy))))
    (else
      (Timeline|Timeline_0 PlayFromStart
        (:Update
          (Replication|UpdateLocation self))))))

(fn ConstructionScript)

(fn InitAttachment)

(fn GetInterpolatedLocation
  (params (Target :type Actor%20Object%20Reference))
  (return (Math|Vector|Lerp(Vector) (Transformation|GetActorLocation Target) (Variables|Replication|GetReplicatedLocation) (* (Utilities|Time|GetWorldDeltaSeconds) 1e+01))))

(fn SpawnProxy
  (Components|DestroyComponent (Variables|Default|GetFloatingPawnMovement))
  (Development|SetHiddeninGame (Variables|Default|GetCube) true true)
  (bind _returnvalue (Game|SpawnActorfromClass "/Game/SolarDefender/Blueprints/Pawns/BP_PawnProxy.BP_PawnProxy_C" (Transformation|GetActorTransform) "AlwaysSpawn" 0 0))
  (Variables|BP_PlayerPawn_C|SetProxy self _returnvalue))

(fn UpdateLocation
  (params (Representative :type Actor%20Object%20Reference))
  (LocalVariables|SetInterpolatedLocation (Replication|GetInterpolatedLocation Representative))
  (if (> (Class|KismetMathLibrary|VectorDistanceSquared (Variables|Replication|GetReplicatedLocation) (LocalVariables|GetInterpolatedLocation)) 1e+03)
    (Transformation|SetActorLocation Representative (LocalVariables|GetInterpolatedLocation) false false)))